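; HUD Blueprint that runs a countdown game session and draws the remaining time and score on screen.
; BeginPlay calls StartGame, which resets score, time and state flags, then starts a looping one-second timer that decrements Time and sets GameOver at zero.
; Collected increments the score and ClockCollected adds bonus time, so game state lives in the HUD itself.
; DrawHUD renders both values as text.
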(event `self.ReceiveDrawHUD`
  (params (SizeX :type Integer) (SizeY :type Integer))
  ;[1 1 1] Draw text - TOP time, BOTTOM score
  (`self.DrawText` (`KismetStringLibrary.Concat_StrStr` "Time remaining: " (`KismetStringLibrary.Conv_IntToString` (`self.time`))) (struct :`A` 1) 10.0 10.0 "/Game/Fonts/AGrazingMace-BgVB_Font.AGrazingMace-BgVB_Font" 2.5)
  (`self.DrawText` (`KismetStringLibrary.Concat_StrStr` "Score: " (`KismetStringLibrary.Conv_IntToString` (`self.score`))) (struct :`A` 1) 10.0 45.0 "/Game/Fonts/AGrazingMace-BgVB_Font.AGrazingMace-BgVB_Font" 2.5))

(event `Timer`
  ;[0.7327 0.9336 1] Timer - decrements timer by 1 and checks if gameOver
  (bind _result (`/Engine/EditorBlueprintResources/StandardMacros.DecrementInt` (`self.time`))
    (:`  `
      (if (<= _result 0)
        (set `self.gameOver` true)
        (`KismetSystemLibrary.K2_ClearTimer` null "Timer")))))

(event `self.ReceiveBeginPlay`
  (`self.StartGame`))

(fn `ClockCollected`
  (set `self.time` (+ (`self.time`) 10)))

(fn `Collected`
  (`/Engine/EditorBlueprintResources/StandardMacros.IncrementInt` (`self.score`)))

(fn `UserConstructionScript`)