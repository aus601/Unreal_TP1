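; Collectible actor that notifies the game HUD and destroys itself when another actor overlaps it.
; On overlap it casts the first player's HUD to TP_GameHUD and calls Collected before destruction, without checking which actor overlapped.
; The construction script applies a configurable mesh and rotating-movement settings (rate, pivot translation, local-space flag), so each instance can have its own look and spin.
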(event `self.ReceiveActorBeginOverlap`
  (params (OtherActor :type "Actor Object Reference"))
  ;[1 1 1] destroy upon collection
  (bind _astp_game_hud (cast `/Game/Blueprints/TP_GameHUD` (`PlayerController.GetHUD` (`GameplayStatics.GetPlayerController` 0))))
  (bind _output_get (set `self.CollectibleGameHUD` _astp_game_hud))
  (`/Game/Blueprints/TP_GameHUD.Collected` _output_get)
  (`self.K2_DestroyActor`))

(fn `UserConstructionScript`
  (bind _rotatingmovement (`self.RotatingMovement`))
  ;[1 1 1] rotate float movement
  (`StaticMeshComponent.SetStaticMesh` (`self.StaticMesh`) (`self.Mesh`))
  (set `RotatingMovementComponent.RotationRate` (`self.Rotation Rate`) _rotatingmovement)
  (set `RotatingMovementComponent.PivotTranslation` (`self.Pivot Translation`) _rotatingmovement)
  (set `RotatingMovementComponent.bRotationInLocalSpace` (`self.Rotation in Local Space`) _rotatingmovement))